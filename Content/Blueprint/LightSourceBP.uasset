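; Light source Blueprint that slowly dims its LightComponent during play.
; Each Tick subtracts a small fixed step from intensity until it falls below a low floor, with no delta-time scaling, so the fade rate depends on frame rate.
; Indirect lighting intensity drops by the same step only while the main fade runs and its value stays at or above its own higher floor.
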(event `self.ReceiveTick`
  (params (DeltaSeconds :type "Float (single-precision)"))
  (if (>= (`LightComponentBase.Intensity` (`self.LightComponent`)) 0.1)
    (`LightComponent.SetIntensity` (`self.LightComponent`) (- (`LightComponentBase.Intensity` (`self.LightComponent`)) 0.001))
    (if (>= (`LightComponentBase.IndirectLightingIntensity` (`self.LightComponent`)) 1.0)
      (`LightComponent.SetIndirectLightingIntensity` (`self.LightComponent`) (- (`LightComponentBase.IndirectLightingIntensity` (`self.LightComponent`)) 0.001)))))

(fn `UserConstructionScript`)