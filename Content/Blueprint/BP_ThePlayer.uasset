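; Player pawn Blueprint handling night vision, flashlights, minimap and injury feedback.
; Night vision swaps camera post-process settings, toggles a directional light set and overlay UI, and drains a battery on Tick until forced off.
; Flashlight input picks rifle-mounted or standalone lights by rifle visibility, syncing infrared counterparts with night vision; key 1 switches them off.
; The map key toggles minimap and marker widgets, while Tick selects injured noise by health thresholds.
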(event `self.ReceiveBeginPlay`
  ;[1 1 1] Add Map
  (set `CameraComponent.PostProcessSettings` (`self.DefaultPost`) (`self.FPSCamera`))
  (set `self.MaxBattery` (`self.BatteryLife`))
  (bind _returnvalue (`|CreateWidget` "/Game/UI/MiniMap/MiniMapWidget.MiniMapWidget_C"))
  (set `self.MiniMap` _returnvalue)
  (`UserWidget.AddToViewport` _returnvalue 0)
  (`Widget.SetVisibility` _returnvalue "Hidden")
  ;[1 1 1] UI
  (bind _returnvalue_2 (`|CreateWidget` "/Game/UI/Battery/NightVisionWidget.NightVisionWidget_C"))
  (bind _output_get (set `self.NV UI` _returnvalue_2))
  (`UserWidget.AddToPlayerScreen` _output_get 0)
  (`Widget.SetVisibility` _returnvalue_2 "Hidden")
  (bind _returnvalue_3 (`|CreateWidget` "/Game/UI/Health/HealthWidget.HealthWidget_C"))
  (`UserWidget.AddToPlayerScreen` _returnvalue_3 0))

(event `InputAction|NightVision`
  (params (Key :type "Key Structure"))
  (bind _nv_ui (`self.NV UI`))
  (bind _fpscamera (`self.FPSCamera`))
  ;[1 1 1] Night vision on / off
  (:`Pressed`
    (if (> (`self.BatteryLife`) 0.0)
      (`/Engine/EditorBlueprintResources/StandardMacros.FlipFlop`
        (:`A`
          (`Widget.SetVisibility` _nv_ui "Visible")
          (set `CameraComponent.PostProcessSettings` (`self.NightVisionTest`) _fpscamera))
        (:`B`
          (`Widget.SetVisibility` _nv_ui "Hidden")
          (set `CameraComponent.PostProcessSettings` (`self.DefaultPost`) _fpscamera)))
      (`SceneComponent.ToggleVisibility` (`self.DirectionalLight`) false)
      (`SceneComponent.ToggleVisibility` (`self.DirectionalLight1`) false)
      (`SceneComponent.ToggleVisibility` (`self.DirectionalLight2`) false)
      (`SceneComponent.ToggleVisibility` (`self.DirectionalLight3`) false)
      (`SceneComponent.ToggleVisibility` (`self.DirectionalLight4`) false)
      (if (`SceneComponent.IsVisible` (`self.FPSRifleMesh`))
        (`SceneComponent.SetVisibility` (`self.Beam`) true false)))))

(event `InputAction|MapToggle`
  (params (Key :type "Key Structure"))
  (bind _minimap (`self.MiniMap`))
  ;[1 1 1] Toggle Map
  (:`Pressed`
    (`/Engine/EditorBlueprintResources/StandardMacros.FlipFlop`
      (:`A`
        (`Widget.SetVisibility` _minimap "Visible")
        (bind _foundwidgets (`WidgetBlueprintLibrary.GetAllWidgetsOfClass` "/Game/UI/MiniMap/MarkerWidget.MarkerWidget_C"))
        (for _array_element _foundwidgets
          (`Widget.SetVisibility` _array_element "Visible")))
      (:`B`
        (`Widget.SetVisibility` _minimap "Hidden")
        (bind _foundwidgets_2 (`WidgetBlueprintLibrary.GetAllWidgetsOfClass` "/Game/UI/MiniMap/MarkerWidget.MarkerWidget_C"))
        (for _array_element_2 _foundwidgets_2
          (`Widget.SetVisibility` _array_element_2 "Hidden"))))))

(event `InputAction|Flashlight`
  (params (Key :type "Key Structure"))
  ;[1 1 1] Flashlight on / off
  (:`Pressed`
    (if (`SceneComponent.IsVisible` (`self.FPSRifleMesh`))
      (`SceneComponent.ToggleVisibility` (`self.M600`) false)
      (if (`SceneComponent.IsVisible` (`self.DirectionalLight4`))
        (`SceneComponent.ToggleVisibility` (`self.m600ir`) false))
      (else
        (`SceneComponent.ToggleVisibility` (`self.SpotLight`) false)
        (if (`SceneComponent.IsVisible` (`self.DirectionalLight4`))
          (`SceneComponent.ToggleVisibility` (`self.FlashlightNV`) false))))))

(event `InputAction|NightVision`
  (params (Key :type "Key Structure"))
  ;[1 1 1] Infared light from flashlights
  (:`Pressed`
    (if (`SceneComponent.IsVisible` (`self.FPSRifleMesh`))
      (if (`SceneComponent.IsVisible` (`self.M600`))
        (`SceneComponent.ToggleVisibility` (`self.m600ir`) false))
      (elif (`SceneComponent.IsVisible` (`self.SpotLight`))
        (`SceneComponent.ToggleVisibility` (`self.FlashlightNV`) false)))))

(event `self.ReceiveTick`
  (params (DeltaSeconds :type "Float (single-precision)"))
  ;[1 1 1] Tick
  (set `self.PlayerPosition` (`self.K2_GetActorLocation` (`GameplayStatics.GetPlayerPawn` 0)))
  (bind _asbp_the_player (cast `/Game/Blueprint/BP_ThePlayer` (`GameplayStatics.GetPlayerPawn` 0)))
  (bind _returnvalue (`self.getHealth` _asbp_the_player))
  (if (< _returnvalue 75)
    (`ActorComponent.Activate` (`self.InjuredNoise`) false)
    (if (< _returnvalue 35)
      (`ActorComponent.Activate` (`self.InjuredNoiseBad`) false)
      (`ActorComponent.Deactivate` (`self.InjuredNoise`)))
    (else
      (`ActorComponent.Deactivate` (`self.InjuredNoise`))
      (`ActorComponent.Deactivate` (`self.InjuredNoiseBad`))))
  (if (`SceneComponent.IsVisible` (`self.DirectionalLight`))
    (bind _output_get (set `self.BatteryLife` (- (`self.BatteryLife`) 0.001)))
    (if (<= _output_get 0.0)
      (`SceneComponent.SetVisibility` (`self.DirectionalLight`) false false)
      (`SceneComponent.SetVisibility` (`self.DirectionalLight1`) false false)
      (`SceneComponent.SetVisibility` (`self.DirectionalLight2`) false false)
      (`SceneComponent.SetVisibility` (`self.DirectionalLight3`) false false)
      (`SceneComponent.SetVisibility` (`self.DirectionalLight4`) false false)
      (`SceneComponent.SetVisibility` (`self.Overlay`) false false)
      (`Widget.SetVisibility` (`self.NV UI`) "Hidden")
      (set `CameraComponent.PostProcessSettings` (`self.DefaultPost`) (`self.FPSCamera`)))
    (`KismetSystemLibrary.PrintText` (`KismetTextLibrary.Conv_DoubleToText` _output_get "HalfToEven") true true (struct :`G` 0.66 :`B` 1.0 :`A` 1.0) 0.0)))

(event `Key|One`
  (params (Key :type "Key Structure"))
  ;[1 1 1] Truning off flashlights when weapons switch
  (:`Pressed`
    (`SceneComponent.SetVisibility` (`self.m600ir`) false false)
    (`SceneComponent.SetVisibility` (`self.M600`) false false)
    (`SceneComponent.SetVisibility` (`self.SpotLight`) false false)
    (`SceneComponent.SetVisibility` (`self.FlashlightNV`) false false)))

(fn `UserConstructionScript`)